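; Test copy of an enemy actor that takes damage, flashes when hit and is destroyed when its health component reports so.
; BeginPlay registers the actor as owner of its health bar widget.
; AttackThis ignores same-class attackers, sets Attacked, damages health, and briefly swaps material slot 0 to a damage material before restoring the originals.
; Attack query functions expose the attack box and return false for CanIAttackThis and ShieldThis.
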(event `self.ReceiveBeginPlay`
  ;[1 1 1] Инициализация параметров врага
  (bind _aswbp_health_bar (cast `/Game/Widgets/WBP_HealthBar` (`WidgetComponent.GetWidget` (`self.WBP_Healthbar`))))
  (`/Game/Widgets/WBP_HealthBar.Set Owner Actor` _aswbp_health_bar self))

(event `self.AttackThis`
  (params (Damage :type "Float (double-precision)") (`Attack Causer` :type "Actor Object Reference"))
  ;[1 1 1] Получение урона и уничтожение пешки
  (if (!= (`GameplayStatics.GetObjectClass` `Attack Causer`) (`GameplayStatics.GetObjectClass` self))
    (set `self.Attacked` true)
    (bind _isdead (`/Game/Components/CBP_HealthComponent.Damage Health` (`self.CBP_HealthComponent`) Damage))
    (if _isdead
      (`self.K2_DestroyActor`)
      (else
        (set `self.Original Material` (`MeshComponent.GetMaterials` (`self.Mesh`)))
        (`PrimitiveComponent.CreateDynamicMaterialInstance` (`self.Mesh`) 0 "/Game/LevelPrototyping/Materials/ActorDamaged.ActorDamaged" "None")
        (`KismetSystemLibrary.Delay` 0.1)
        (for (_array_element _array_index) (`self.Original material`)
          (`PrimitiveComponent.SetMaterial` (`self.Mesh`) _array_index _array_element))))))

(fn `CanIAttackThis?`
  (returns (`Yes You Can` :type Boolean))
  (return false))

(fn `Get Attack Box`
  (returns (`Attack Box` :type "BoxComponent Object Reference"))
  (return (`self.AttackBox`)))

(fn `ShieldThis`
  (params (Attacker :type "BoxComponent Object Reference"))
  (returns (Block :type Boolean))
  (return false))

(fn `UserConstructionScript`)