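; BP_Game_GameModeBase is a game mode Blueprint that tracks active quests and provides helpers for info UI and enemy counting.
; The AddQuest event appends the given quest to the active quest array.
; CreateInfoWidget spawns a WBP_Info widget, anchors it in the viewport and activates it with placeholder test text.
; CountEnemiesOfClass returns the number of actors of a given class via GetAllActorsOfClass.
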(event `/Game/ThirdPerson/Blueprints/Interfaces/IBP_Quest_System.Add Quest`
  (params (`This Quest` :type "/Game/ThirdPerson/Blueprints/Structures/ST_Quest Structure"))
  (`KismetArrayLibrary.Array_Add` (`self.Array of Active Quests`) `This Quest`))

(fn `Count Enemies of Class`
  (params (ActorClass :type "Actor Class Reference"))
  (returns (`Enemy Counter` :type Integer))
  (bind _outactors (`GameplayStatics.GetAllActorsOfClass` ActorClass))
  (return (`KismetArrayLibrary.Array_Length` _outactors)))

(fn `Create Info Widget`
  (locals (`Local Anchors` :type "Anchors Structure" :default (struct :`Minimum` (0.5 0.4) :`Maximum` (0.5 0.4))) (`Local Info Widget` :type "/Game/Widgets/WBP_Info Object Reference"))
  (bind _returnvalue (`|CreateWidget` "/Game/Widgets/WBP_Info.WBP_Info_C"))
  (bind _output_get (set `local.Local Info Widget` _returnvalue))
  (`UserWidget.SetAnchorsInViewport` _output_get (`local.Local Anchors`))
  (`UserWidget.AddToViewport` (`local.Local Info Widget`) 0)
  (`/Game/Widgets/WBP_Info.Activate` (`local.Local Info Widget`) "Test Text"))

(fn `UserConstructionScript`)