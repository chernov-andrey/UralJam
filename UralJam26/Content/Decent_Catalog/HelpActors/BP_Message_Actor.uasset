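; BP_Message_Actor is a trigger actor that shows the player a text message and pauses the game the first time they enter it.
; On BeginPlay it creates a hidden WBP_Message widget with its configured text.
; Overlap by an actor tagged Player reveals the widget once, with unpausing left to the widget's own logic.
; It also calls ThisActorAction, an empty hook receiving the overlapping actor.
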(event `self.ReceiveBeginPlay`
  ;[1 1 1] Создание виджета, добавление его во вьевпорт, задание текста виджету и сокрытие виджета.
  (bind _returnvalue (`|CreateWidget` "/Game/Decent_Catalog/GUI/WBP_Message.WBP_Message_C"))
  (bind _output_get (set `self.As WBP Message` _returnvalue))
  (`/Game/Decent_Catalog/GUI/WBP_Message.Set Text to Textblock` _output_get (`self.This Message Text`))
  (`Widget.SetVisibility` (`self.As WBP Message`) "Hidden")
  (`UserWidget.AddToViewport` (`self.As WBP Message`) 0))

(event `self.ReceiveActorBeginOverlap`
  (params (OtherActor :type "Actor Object Reference"))
  ;[1 1 1] Если игрок вошёл в зону действия триггера, то показываем ему виджет и ставим игру на паузу (пауза отжимается в логике самого виджета)
  (if (`self.ActorHasTag` OtherActor "Player")
    (set `self.Other Actor` OtherActor)
    (if (not (`self.Was shown?`))
      (`Widget.SetVisibility` (`self.As WBP Message`) "Visible")
      (`GameplayStatics.SetGamePaused` true)
      (`self.This Actor Action` (`self.Other Actor`))
      (set `self.Was shown?` true))))

(fn `This Actor Action`
  (params (`Overlapped Actor` :type "Actor Object Reference")))

(fn `UserConstructionScript`)