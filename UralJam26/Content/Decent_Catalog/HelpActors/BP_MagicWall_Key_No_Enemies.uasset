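; Magic wall key variant that destroys itself once every tracked enemy in the level is dead.
; On BeginPlay it counts all actors of a given class and binds to each BP_Enemy health component's death dispatcher.
; Each death decrements the counter and checks the overridden RequiermentsToUnlock, which passes when the count reaches zero or below.
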(event `self.ReceiveBeginPlay`
  (`parent.ReceiveBeginPlay`)
  (bind _outactors (`GameplayStatics.GetAllActorsOfClass` (`self.Actor Class`)))
  (set `self.Counter` (`KismetArrayLibrary.Array_Length` _outactors))
  (for _array_element _outactors
    (bind _asbp_enemy (cast `/Game/ThirdPerson/AI/MasterEnemy/BP_Enemy` _array_element))
    (add `/Game/Components/CBP_HealthComponent.Dead_Dispatch` (`/Game/ThirdPerson/AI/MasterEnemy/BP_Enemy.CBP_HealthComponent` _asbp_enemy) (delegate `Dead Dispatch Helper`))))

(event `Dead Dispatch Helper`
  (`/Engine/EditorBlueprintResources/StandardMacros.DecrementInt` (`self.Counter`)
    (:`  `
      (bind _unlock (`self.Requierments to Unlock`))
      (if _unlock
        (`self.K2_DestroyActor`)))))

(fn `Requierments to Unlock`
  (returns (Unlock :type Boolean))
  (`parent.Requierments to Unlock`)
  (return (<= (`self.Counter`) 0)))

(fn `UserConstructionScript`
  (`parent.UserConstructionScript`))