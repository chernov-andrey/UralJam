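; BP_MaxHP_Increaser is a helper actor that permanently raises the player character's maximum health.
; It overrides the parent's ThisActorAction, calls the parent logic, then casts the overlapped actor to BP_MaterCharacter and adds a fixed bonus to its health component's max health.
; An unconnected branch would create an info widget through the game mode, with a note citing poor visibility and animation problems.
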(fn `This Actor Action`
  (params (`Overlapped Actor` :type "Actor Object Reference"))
  (`parent.This Actor Action` `Overlapped Actor`)
  (bind _asbp_mater_character (cast `/Game/ThirdPerson/Blueprints/BP_MaterCharacter` `Overlapped Actor`))
  (bind _cbp_healthcomponent (`/Game/ThirdPerson/Blueprints/BP_MaterCharacter.CBP_HealthComponent` _asbp_mater_character))
  (bind _max_health (`/Game/Components/CBP_HealthComponent.get Max Health` _cbp_healthcomponent))
  (`/Game/Components/CBP_HealthComponent.Set MaxHealth` _cbp_healthcomponent (+ _max_health 20.0)))

(fn `UserConstructionScript`
  (`parent.UserConstructionScript`))