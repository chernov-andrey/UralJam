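; BP_Next_level_trigger is an overlap trigger that moves the game on to the next level after a player choice.
; On overlap it runs the parent's overlap logic and binds a handler to the ChoiceResult event.
; A Left result makes the UralJam game instance save data from the overlapping actor, then launch the stored level with the current hero class.
; SetNextLevel sets that target level name.
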(event `self.ReceiveActorBeginOverlap`
  (params (OtherActor :type "Actor Object Reference"))
  (`parent.ReceiveActorBeginOverlap` OtherActor)
  (add `self.Choice Result` (delegate `Choice Result Helper`)))

(event `Choice Result Helper`
  (bind _as_bp_ural_jam_game_instance (`self.As BP Ural Jam Game Instance`))
  (if (`self.Left`)
    ;[1 1 1] Запуск следующего уровня
    (`/Game/Decent_Catalog/GameSetting/BP_UralJam_GameInstance.Save Data` (`self.As BP Ural Jam Game Instance`) (`self.Other Actor`))
    (`UralJam_GameInstance.Launch_NewLevel` _as_bp_ural_jam_game_instance (`self.New Level Name`) (`UralJam_GameInstance.CurrentClassHero` _as_bp_ural_jam_game_instance))))

(fn `Set NextLevel`
  (params (`New Level Name` :type Name))
  (set `self.New Level Name` `New Level Name`))

(fn `UserConstructionScript`
  (`parent.UserConstructionScript`))