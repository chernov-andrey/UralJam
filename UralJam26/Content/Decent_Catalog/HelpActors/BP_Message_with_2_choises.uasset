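; BP_Message_with_2_choises is a helper actor that shows a two-choice message when an actor tagged Player overlaps it.
; The overlap creates WBP_Message_With_2_Choise, applies the stored text and button labels, adds it to the viewport and binds to its choice event.
; A choice removes the widget, stores Left and calls ChoiceResult.
; Setter functions let the message and both labels be changed.
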(event `self.ReceiveActorBeginOverlap`
  (params (OtherActor :type "Actor Object Reference"))
  ;[1 1 1] Определяем, что близко подошёл игрок
  (if (`self.ActorHasTag` OtherActor "Player")
    (set `self.Other Actor` OtherActor)
    (bind _asbp_ural_jam_game_instance (cast `/Game/Decent_Catalog/GameSetting/BP_UralJam_GameInstance` (`GameplayStatics.GetGameInstance`)))
    (bind _output_get (set `self.As BP Ural Jam Game Instance` _asbp_ural_jam_game_instance))
    (`/Engine/EditorBlueprintResources/StandardMacros.IsValid` _output_get
      (:`Is Valid`
        (bind _returnvalue (`|CreateWidget` "/Game/Decent_Catalog/GUI/WBP_Message_With_2_Choise.WBP_Message_With_2_Choise_C"))
        (bind _output_get_2 (set `self.As WBP_Message_with_2_choise` _returnvalue))
        (`/Game/Decent_Catalog/GUI/WBP_Message_With_2_Choise.Set Owner` _output_get_2 self)
        (`/Game/Decent_Catalog/GUI/WBP_Message_With_2_Choise.Name Button` (`self.As WBP_Message_with_2_choise`) 0 (`self.Button 0`))
        (`/Game/Decent_Catalog/GUI/WBP_Message_With_2_Choise.Name Button` (`self.As WBP_Message_with_2_choise`) 1 (`self.Button 1`))
        (`/Game/Decent_Catalog/GUI/WBP_Message_With_2_Choise.Set Text to Textblock` (`self.As WBP_Message_with_2_choise`) (`self.Message - Mission Complete`))
        (`UserWidget.AddToViewport` (`self.As WBP_Message_with_2_choise`) 0)
        (add `/Game/Decent_Catalog/GUI/WBP_Message_With_2_Choise.Choise Made` (`self.As WBP_Message_with_2_choise`) (delegate `Choise Made Helper`))))))

(event `Choise Made Helper`
  (params (Left :type Boolean))
  (`Widget.RemoveFromParent` (`self.As WBP_Message_with_2_choise`))
  (set `self.Left` Left)
  (`self.Choice Result`))

(fn `Name Button Accept`
  (params (`Button Accept` :type String))
  (set `self.Button 0` `Button Accept`))

(fn `Name Button Decline`
  (params (`Button Decline` :type String))
  (set `self.Button 1` `Button Decline`))

(fn `Set Text to Message`
  (params (`Message Text` :type String))
  (set `self.Message - Mission Complete` `Message Text`))

(fn `UserConstructionScript`)