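; BP_Box_Splinters is a short-lived actor, by its name the debris of a broken box, that removes itself after a countdown.
; Each Tick subtracts delta time from TimeToLive and destroys the actor once it reaches zero or below.
; SetTimeToLive provides a setter for the remaining lifetime, while the construction script only calls its parent.
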(event `self.ReceiveTick`
  (params (DeltaSeconds :type "Float (single-precision)"))
  (`parent.ReceiveTick` DeltaSeconds)
  (bind _output_get (set `self.Time to Live` (- (`self.Time to Live`) DeltaSeconds)))
  (if (<= _output_get 0.0)
    (`self.K2_DestroyActor`)))

(fn `Set TimeToLive`
  (params (`Time To Live` :type "Float (double-precision)"))
  (set `self.Time to Live` `Time To Live`))

(fn `UserConstructionScript`
  (`parent.UserConstructionScript`))